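; AudioData is a Blueprint for song audio analysis that, as wired, only tracks a playback time through ResetSong and SetSongInTime.
; Disconnected chains would play a song, advance the time and write loudness to the Volume parameter of a Material Parameter Collection.
; GetLoudAndAmplitude is a stub: its Constant-Q and normalized loudness lookups are unconnected, and BeginPlay and Tick are empty.
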(event `self.ReceiveBeginPlay`)

(event `self.ReceiveTick`
  (params (DeltaSeconds :type "Float (single-precision)")))

(event `ResetSong`
  (`self.SetSongInTime` 0.0))

(event `SetSongInTime`
  (params (NewTime :type "Float (double-precision)"))
  (set `self.currentSongTime` NewTime))

(fn `UserConstructionScript`)